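; Game mode for a block-breaking game that tracks lives, score, game over and level completion.
; On BeginPlay it creates the HUD and resets state, then pushes score and life changes to it, clamping score at zero and penalizing lost lives.
; Every Tick counts actors tagged "Block" to detect a cleared level.
; Game over and level clear each play a sound, then reload Level1 after a delay.
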(event Custom|Reset
  (bind _maxlives (Variables|Default|GetMaxLives))
  (bind _hud (Variables|Default|GetHUD))
  ;[1 1 1] Reset Game
  (Variables|Default|SetLives _maxlives)
  (Variables|/Game/Blueprints/HUD.HUD_C|SetLives _hud _maxlives)
  (Variables|/Game/Blueprints/HUD.HUD_C|SetPoints _hud 0)
  (Variables|Default|SetCurrentPoints 0)
  (Variables|Default|SetGameOver? false))

(event Custom|UpdateScore
  (params (Points :type Integer))
  ;[1 1 1] Update Score
  (if (<= (+ Points (Variables|Default|GetCurrentPoints)) 0)
    (Variables|Default|SetCurrentPoints 0)
    (else
      (Variables|Default|SetCurrentPoints (+ Points (Variables|Default|GetCurrentPoints)))))
  (Variables|/Game/Blueprints/HUD.HUD_C|SetPoints (Variables|Default|GetHUD) (Variables|Default|GetCurrentPoints)))

(event Custom|LifeLost
  ;[1 1 1] LifeLost
  (CallFunction|UpdateScore -500)
  (if (<= (Variables|Default|GetLives) 0)
    (CallFunction|GameOver)
    (else
      (bind _output_get (Variables|Default|SetLives (- (Variables|Default|GetLives) 1)))
      (Variables|/Game/Blueprints/HUD.HUD_C|SetLives (Variables|Default|GetHUD) _output_get))))

(event Custom|GameOver
  ;[1 1 1] Game Over
  (Variables|Default|SetGameOver? true)
  (Audio|PlaySound2D "/Game/Audio/GameOver.GameOver" 1.0 1.0 0.0 0 0)
  (Utilities|FlowControl|Delay 5.0)
  (Game|OpenLevel(byName) "Level1"))

(event Custom|BlocksRemainigCheck
  ;[1 1 1] BlockRemainingCheck
  (bind _outactors (Actor|GetAllActorswithTag "Block"))
  (bind _output_get (Variables|Default|SetBlocksRemaining (Utilities|Array|Length _outactors)))
  (Development|PrintString (Utilities|String|ToString(Integer) _output_get))
  (if (<= _output_get 0)
    (CallFunction|LevelClear)))

(event Custom|LevelClear
  ;[1 1 1] LevelClear
  (Variables|Default|SetLevelClear? true)
  (Audio|PlaySound2D "/Game/Audio/LevelCompleted.LevelCompleted" 1.0 1.0 0.0 0 0)
  (Utilities|FlowControl|Delay 5.0)
  (Game|OpenLevel(byName) "Level1"))

(event EventBeginPlay
  ;[1 1 1] Add HUD
  (bind _returnvalue (UserInterface|CreateWidget "/Game/Blueprints/HUD.HUD_C"))
  (bind _output_get (Variables|Default|SetHUD _returnvalue))
  (UserInterface|Viewport|AddtoViewport _output_get 0)
  (CallFunction|Reset))

(event EventTick
  (params (DeltaSeconds :type Float%20%28single-precision%29))
  ;[1 1 1] BlockRemainingCheck
  (bind _outactors (Actor|GetAllActorswithTag "Block"))
  (bind _output_get (Variables|Default|SetBlocksRemaining (Utilities|Array|Length _outactors)))
  (Development|PrintString (Utilities|String|ToString(Integer) _output_get))
  (if (<= _output_get 0)
    (CallFunction|LevelClear)))

(fn ConstructionScript)